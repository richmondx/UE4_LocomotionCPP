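; Pawn Blueprint that relays locomotion state and movement settings to its animation instance.
; Rotation mode, gait and aiming events call the parent implementation, then forward the value through Blueprint Interface messages.
; Walking, running and sprinting speed events only forward to the animation instance, with no parent call.
; An interface event also passes rotation amounts to AddCharacterRotation.
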(event `self.ReceiveBeginPlay`)

(event `/Game/Blueprints/BPI_Locomotion.AddCharacterRotation_BPI`
  (params (AddAmount :type "Rotator Structure"))
  (`self.AddCharacterRotation` AddAmount))

(event `self.OnRotationModeChanged`
  (`parent.OnRotationModeChanged`)
  (message `/Game/Blueprints/BPI_Locomotion.Set Locomotion_RotationMode BPI` (`self.GetAnimInstance`) (`self.PlayerRotationMode`)))

(event `self.SetGaitEvent`
  (params (Gait :type "ELocomotion_Gait Enum" :default "Walking"))
  (`parent.SetGaitEvent` Gait)
  (message `/Game/Blueprints/BPI_Locomotion.Set Locomotion_Gait BPI` (`self.GetAnimInstance`) Gait))

(event `self.SetAimingModeEvent`
  (params (NewAiming :type Boolean))
  (`parent.SetAimingModeEvent` NewAiming)
  (message `/Game/Blueprints/BPI_Locomotion.Set Locomotion_Aiming BPI` (`self.GetAnimInstance`) NewAiming))

(event `self.SetRotationModeEvent`
  (params (RotMode :type "ELocomotion_RotationMode Enum" :default "LookingDirection"))
  (`parent.SetRotationModeEvent` RotMode)
  (message `/Game/Blueprints/BPI_Locomotion.Set Locomotion_RotationMode BPI` (`self.GetAnimInstance`) RotMode))

(event `self.SetWalkingSpeedEvent`
  (params (NewWalkingSpeed :type "Float (single-precision)"))
  (message `/Game/Blueprints/BPI_Locomotion.Set WalkingSpeed BPI` (`self.GetAnimInstance`) NewWalkingSpeed))

(event `self.SetRunningSpeedEvent`
  (params (NewRunningSpeed :type "Float (single-precision)"))
  (message `/Game/Blueprints/BPI_Locomotion.Set RunningSpeed BPI` (`self.GetAnimInstance`) NewRunningSpeed))

(event `self.SetSprintingSpeedEvent`
  (params (NewSprintingSpeed :type "Float (single-precision)"))
  (message `/Game/Blueprints/BPI_Locomotion.Set SprintingSpeed BPI` (`self.GetAnimInstance`) NewSprintingSpeed))

(fn `UserConstructionScript`)